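; NPC girl character in a Guardian game mode whose death ends the game.
; Weapon Attack applies fixed damage to her from the given instigator, but only damage from a KataAIController lowers Health.
; Health changes are relayed to GuardianGameMode; at zero, ServerDeath calls MultiDeath for the fall montage, then EndGame follows a delay.
; IsDeath is set only after that delay and EndGame call.
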(event Custom|MultiDeath
  (Animation|PlayAnimMontage "/Game/BluePrint/NPC/Animation/Falling_Back_Death_Montage.Falling_Back_Death_Montage" 1.0 "None"))

(event Custom|ServerDeath
  (CallFunction|MultiDeath))

(event Custom|ServerUpdateNpcHealth
  (params (Health :type Float%20%28single-precision%29))
  (bind _asguardian_game_mode (Utilities|Casting|CastToGuardianGameMode (Game|GetGameMode)))
  (Default|UpdateNpcHealth _asguardian_game_mode Health))

(event Game|Damage|EventAnyDamage
  (params (Damage :type Float%20%28single-precision%29) (DamageType :type Damage%20Type%20Object%20Reference) (InstigatedBy :type Controller%20Object%20Reference) (DamageCauser :type Actor%20Object%20Reference))
  (Utilities|Casting|CastToKataAIController InstigatedBy
    (:then
      (bind _output_get (Variables|Default|SetHealth (- (Variables|Default|GetHealth) Damage)))
      (CallFunction|ServerUpdateNpcHealth _output_get)
      (if (<= (Variables|Default|GetHealth) 0.0)
        (if (not (Variables|Default|GetIsDeath))
          (CallFunction|ServerDeath)
          (Utilities|FlowControl|Delay 2.6)
          (bind _asguardian_game_mode (Utilities|Casting|CastToGuardianGameMode (Game|GetGameMode)))
          (Default|EndGame _asguardian_game_mode)
          (Variables|Default|SetIsDeath true))))
    (:CastFailed
      (Utilities|Casting|CastToShooterAIController InstigatedBy))))

(fn ConstructionScript)

(fn WeaponAttack
  (params (Killer :type Kata%20AI%20Controller%20Object%20Reference))
  (Game|Damage|ApplyDamage self 1e+01 Killer 0)
  (return true))