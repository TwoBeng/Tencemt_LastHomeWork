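; Deathmatch game mode that runs a timed round, spawns players and keeps their scores.
; The first login gathers PlayerStarts and starts a one-second countdown, pushed to every controller until the round ends.
; Spawn requests cycle through those points round-robin to spawn Attacker characters.
; A controller-keyed map holds each player's data; kill and death events rewrite entries and send the updated scoreboard to all players.
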(event Custom|UpdateScore
  (bind _playergamedatamap (Variables|Default|GetPlayerGameDataMap))
  ;[1 1 1] UpdateScore
  (bind _keys (Utilities|Map|Keys _playergamedatamap))
  (for _array_element _keys
    (bind _values (Utilities|Map|Values _playergamedatamap))
    (Default|UpdateScore _array_element _values)))

(event Custom|UpdateTime
  ;[1 1 1] UpdateTime
  (bind _outactors (Actor|GetAllActorsOfClass "/Script/Engine.PlayerStart"))
  (Variables|Default|SetCharacter%20Spawn%20Points _outactors)
  (bind _returnvalue (Utilities|Time|SetTimerbyEvent (delegate Custom|DownTime) 1.0 true))
  (Variables|Default|SetDownTimeHandler _returnvalue))

(event Custom|Kill%20Player
  (params (KillPlayerController :type My%20Player%20Controller%20BP%20Object%20Reference))
  (bind _playergamedatamap (Variables|Default|GetPlayerGameDataMap))
  (bind _playergamedatamap_2 (Variables|Default|GetPlayerGameDataMap))
  (bind _value (Utilities|Map|Find _playergamedatamap_2 KillPlayerController))
  (bind (_playername _playerscore _killnum _deathnum) (Utilities|Struct|BreakDeathMatchPlayerData _value))
  ;[1 1 1] UpdateScore
  (bind _output_get (Variables|Default|SetKill%20Player%20Score (+ _playerscore 15)))
  (bind _output_get_2 (Variables|Default|SetKill%20Player%20Name _playername))
  (bind _output_get_3 (Variables|Default|SetKiller%20Kill%20Num (+ _killnum 1)))
  (bind _output_get_4 (Variables|Default|SetKiller%20Death%20Num _deathnum))
  (Utilities|Map|Remove _playergamedatamap KillPlayerController)
  (Utilities|Map|Add _playergamedatamap KillPlayerController (Utilities|Struct|MakeDeathMatchPlayerData _output_get_2 _output_get _output_get_3 _output_get_4))
  (CallFunction|UpdateScore))

(event Custom|DownTime
  ;[1 1 1] UpdateTime
  (Variables|Default|SetRoundTime (- (Variables|Default|GetRoundTime) 1))
  (bind _keys (Utilities|Map|Keys (Variables|Default|GetPlayerGameDataMap)))
  (for _array_element _keys
    (Default|ClientUpdateTime _array_element (Variables|Default|GetRoundTime)))
  (if (<= (Variables|Default|GetRoundTime) 0)
    (Utilities|Time|ClearandInvalidateTimerbyHandle (Variables|Default|GetDownTimeHandler))
    (CallFunction|EndGame)))

(event Custom|SelfDeath
  (params (DeathPlayerController :type My%20Player%20Controller%20BP%20Object%20Reference))
  (bind _playergamedatamap (Variables|Default|GetPlayerGameDataMap))
  (bind _playergamedatamap_2 (Variables|Default|GetPlayerGameDataMap))
  (bind _value (Utilities|Map|Find _playergamedatamap DeathPlayerController))
  (bind (_playername _playerscore _killnum _deathnum) (Utilities|Struct|BreakDeathMatchPlayerData _value))
  ;[1 1 1] UpdateScore
  (bind _output_get (Variables|Default|SetDeath%20Player%20Score (- _playerscore 10)))
  (bind _output_get_2 (Variables|Default|SetDeath%20Player%20Name _playername))
  (bind _output_get_3 (Variables|Default|SetDeath%20Player%20Death%20Num (+ _deathnum 1)))
  (bind _output_get_4 (Variables|Default|SetDeath%20Player%20Kill%20Num _killnum))
  (Utilities|Map|Remove _playergamedatamap_2 DeathPlayerController)
  (Utilities|Map|Add _playergamedatamap_2 DeathPlayerController (Utilities|Struct|MakeDeathMatchPlayerData _output_get_2 _output_get _output_get_4 _output_get_3))
  (CallFunction|UpdateScore))

(event Custom|EndGame
  ;[1 1 1] EndGame
  (bind _keys (Utilities|Map|Keys (Variables|Default|GetPlayerGameDataMap)))
  (for _array_element _keys
    (Default|ClientEndGame _array_element)))

(event Custom|RequestSpawn
  (params (PlayerController :type My%20Player%20Controller%20BP%20Object%20Reference))
  ;[1 1 1] Login && Spawn Player
  (Default|SpawnPlayerCharater PlayerController "/Game/BluePrint/Player/Attacker.Attacker_C" (Transformation|GetActorTransform (Utilities|Array|Get(acopy) (Variables|Default|GetCharacter%20Spawn%20Points) (Variables|Default|GetSpawnIndex))))
  (Variables|Default|SetSpawnIndex (+ (Variables|Default|GetSpawnIndex) 1))
  (if (>= (Variables|Default|GetSpawnIndex) (Utilities|Array|Length (Variables|Default|GetCharacter%20Spawn%20Points)))
    (Variables|Default|SetSpawnIndex 0)))

(event EventPostLogin
  (params (NewPlayer :type Player%20Controller%20Object%20Reference))
  ;[1 1 1] Login && Spawn Player
  (bind _asmy_player_controller_bp (Utilities|Casting|CastToMyPlayerController_BP NewPlayer))
  (if (Variables|Default|GetIsFirstPerson)
    (Variables|Default|SetIsFirstPerson false)
    (CallFunction|UpdateTime))
  (Default|StartSpawnPlayerCharacter _asmy_player_controller_bp)
  (Utilities|Map|Add (Variables|Default|GetPlayerGameDataMap) _asmy_player_controller_bp (Utilities|Struct|MakeDeathMatchPlayerData (Utilities|String|StringToName (Utilities|GetObjectName _asmy_player_controller_bp)))))

(fn ConstructionScript)