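; MainMenuController_BP is a player controller for the main menu flow.
; On BeginPlay it creates the W_MainUI widget and adds it to the viewport.
; Pressing Enter removes that widget, shows W_MainMenuUI, switches input to UI-only focused on the new menu, and shows the mouse cursor.
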(event EventBeginPlay
  (bind _returnvalue (UserInterface|CreateWidget "/Game/BluePrint/GameUI/W_MainUI.W_MainUI_C" self))
  (bind _output_get (Variables|Default|SetMainUI _returnvalue))
  (Utilities|IsValid _output_get
    (:Is%20Valid
      (UserInterface|Viewport|AddtoViewport _output_get 0))))

(event Input|KeyboardEvents|Enter
  (params (Key :type Key%20Structure :default "None"))
  (:Pressed
    (Widget|RemovefromParent (Variables|Default|GetMainUI))
    (bind _returnvalue (UserInterface|CreateWidget "/Game/BluePrint/GameUI/W_MainMenuUI.W_MainMenuUI_C" self))
    (UserInterface|Viewport|AddtoViewport _returnvalue 0)
    (Input|SetInputModeUIOnly self _returnvalue "DoNotLock")
    (Variables|Default|SetbShowMouseCursor true)))

(fn ConstructionScript)