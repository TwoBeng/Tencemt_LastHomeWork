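; Game mode for a multiplayer guardian match with a shared life pool, a round countdown and score tracking.
; PostLogin starts the timer for the first player, adds lives, registers player data keyed by controller and spawns a Kata AI.
; Spawns rotate through player starts and consume lives; exhausted lives or time end the game.
; Life, time, health and score changes relay to every controller; other events spawn shooter AI and weapon pickups.
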(event Custom|UpdateScore
  (bind _playergamedatamap (Variables|Default|GetPlayerGameDataMap))
  ;[1 1 1] UpdateScore
  (bind _keys (Utilities|Map|Keys _playergamedatamap))
  (for _array_element _keys
    (bind _values (Utilities|Map|Values _playergamedatamap))
    (Default|UpdateScore _array_element _values)))

(event Custom|UpdateTime
  ;[1 1 1] UpdateTime
  (bind _outactors (Actor|GetAllActorsOfClass "/Script/Engine.PlayerStart"))
  (Variables|Default|SetCharacter%20Spawn%20Points _outactors)
  (bind _returnvalue (Utilities|Time|SetTimerbyEvent (delegate Custom|DownTime) 1.0 true))
  (Variables|Default|SetDownTimeHandler _returnvalue))

(event Custom|UpdateLifeNum
  (params (LifeNum :type Integer))
  (bind _keys (Utilities|Map|Keys (Variables|Default|GetPlayerGameDataMap)))
  (for _array_element _keys
    (Default|ClientUpdateLifeNum _array_element LifeNum)))

(event Custom|SpawnAk47
  (params (Location :type Vector))
  (bind _returnvalue (Game|SpawnActorfromClass "/Game/BluePrint/Weapon/Ak47/Server_Ak47_BP.Server_Ak47_BP_C" (Math|Transform|MakeTransform (.RandomLocation (AI|Navigation|GetRandomReachablePointinRadius Location 1e+02 0 0)) "0, 0, 0" "1,1,1") "Undefined" 0 0))
  (Collision|SetCollisionEnabled (Variables|/Script/Net.WeaponBaseServer|GetSphereCollision _returnvalue) "QueryAndPhysics"))

(event Custom|UpdateNpcHealth
  (params (Health :type Float%20%28single-precision%29))
  (bind _keys (Utilities|Map|Keys (Variables|Default|GetPlayerGameDataMap)))
  (for _array_element _keys
    (Development|PrintString "NUm")
    (Default|ClientUpdateNpcHealth _array_element Health)))

(event Custom|Kill%20Player
  (params (KillPlayerController :type Guardian%20Player%20Controller%20BP%20Object%20Reference))
  (bind _playergamedatamap (Variables|Default|GetPlayerGameDataMap))
  (bind _playergamedatamap_2 (Variables|Default|GetPlayerGameDataMap))
  (bind _value (Utilities|Map|Find _playergamedatamap KillPlayerController))
  (bind (_playername _playerscore _killnum _deathnum _health) (Utilities|Struct|BreakDeathMatchPlayerData _value))
  ;[1 1 1] UpdateScore
  (bind _output_get (Variables|Default|SetKill%20Player%20Score (+ _playerscore 15)))
  (bind _output_get_2 (Variables|Default|SetKill%20Player%20Name _playername))
  (bind _output_get_3 (Variables|Default|SetKiller%20Kill%20Num (+ _killnum 1)))
  (bind _output_get_4 (Variables|Default|SetKiller%20Death%20Num _deathnum))
  (bind _output_get_5 (Variables|Default|SetKiller%20Health _health))
  (Utilities|Map|Remove _playergamedatamap_2 KillPlayerController)
  (Utilities|Map|Add _playergamedatamap_2 KillPlayerController (Utilities|Struct|MakeDeathMatchPlayerData _output_get_2 _output_get _output_get_3 _output_get_4 _output_get_5))
  (CallFunction|UpdateScore))

(event Custom|DownTime
  ;[1 1 1] UpdateTime
  (Variables|Default|SetRoundTime (- (Variables|Default|GetRoundTime) 1))
  (bind _keys (Utilities|Map|Keys (Variables|Default|GetPlayerGameDataMap)))
  (for _array_element _keys
    (Default|ClientUpdateTime _array_element (Variables|Default|GetRoundTime)))
  (if (<= (Variables|Default|GetRoundTime) 0)
    (Utilities|Time|ClearandInvalidateTimerbyHandle (Variables|Default|GetDownTimeHandler))
    (CallFunction|EndGame)))

(event Custom|SpawnAIShooter
  (bind _returnvalue (AI|SpawnAIFromClass "/Game/BluePrint/AI/Shooter/Shooter.Shooter_C" "/Game/BluePrint/AI/Shooter/AI/Shooter_BT.Shooter_BT" (.RandomLocation (AI|Navigation|GetRandomReachablePointinRadius (Transformation|GetActorLocation (Utilities|Array|Get(acopy) (Variables|Default|GetCharacter%20Spawn%20Points))) 5e+02 0 0)) "0, 0, 0" false 0))
  (Variables|/Script/Engine.Pawn|SetAIControllerClass _returnvalue "/Game/BluePrint/AI/Shooter/AI/ShooterAIController.ShooterAIController_C"))

(event Custom|EndGame
  ;[1 1 1] EndGame
  (bind _keys (Utilities|Map|Keys (Variables|Default|GetPlayerGameDataMap)))
  (for _array_element _keys
    (Default|ClientEndGame _array_element)))

(event Custom|SpawAIKata
  (bind _returnvalue (AI|SpawnAIFromClass "/Game/BluePrint/AI/Katanami/KataAICharacter.KataAICharacter_C" "/Game/BluePrint/AI/Katanami/AI/KataBT.KataBT" (.RandomLocation (AI|Navigation|GetRandomReachablePointinRadius (Transformation|GetActorLocation (Utilities|Array|Get(acopy) (Variables|Default|GetCharacter%20Spawn%20Points))) 5e+02 0 0)) "0, 0, 0" false 0))
  (Utilities|IsValid _returnvalue
    (:Is%20Valid
      (Variables|/Script/Engine.Pawn|SetAIControllerClass _returnvalue "/Game/BluePrint/AI/Katanami/AI/KataAIController.KataAIController_C"))))

(event Custom|SpawnM4A1
  (params (Location :type Vector))
  (bind _returnvalue (Game|SpawnActorfromClass "/Game/BluePrint/Weapon/M4A1/Server_M4A1_BP.Server_M4A1_BP_C" (Math|Transform|MakeTransform (.RandomLocation (AI|Navigation|GetRandomReachablePointinRadius Location 1e+02 0 0)) "0, 0, 0" "1,1,1") "Undefined" 0 0))
  (Collision|SetCollisionEnabled (Variables|/Script/Net.WeaponBaseServer|GetSphereCollision _returnvalue) "QueryAndPhysics"))

(event Custom|Spawn%20Sniper
  (params (Location :type Vector))
  (bind _returnvalue (Game|SpawnActorfromClass "/Game/BluePrint/Weapon/Sniper/Server_Sniper_BP.Server_Sniper_BP_C" (Math|Transform|MakeTransform (.RandomLocation (AI|Navigation|GetRandomReachablePointinRadius Location 1e+02 0 0)) "0, 0, 0" "1,1,1") "Undefined" 0 0))
  (Collision|SetCollisionEnabled (Variables|/Script/Net.WeaponBaseServer|GetSphereCollision _returnvalue) "QueryAndPhysics"))

(event Custom|Update%20All%20Player%20Health
  (params (PlayerController :type Guardian%20Player%20Controller%20BP%20Object%20Reference) (Health :type Float%20%28single-precision%29))
  (bind _playergamedatamap (Variables|Default|GetPlayerGameDataMap))
  (Variables|Default|SetHealth%20Data (.Value (Utilities|Map|Find _playergamedatamap PlayerController)))
  (Utilities|Map|Remove (Variables|Default|GetPlayerGameDataMap) PlayerController)
  (bind _output_get (Variables|Default|SetHealth%20Data (Utilities|Struct|MakeDeathMatchPlayerData (.playername (Variables|Default|GetHealth%20Data)) (.playerscore (Variables|Default|GetHealth%20Data)) (.killnum (Variables|Default|GetHealth%20Data)) (.deathnum (Variables|Default|GetHealth%20Data)) Health)))
  (Utilities|Map|Add (Variables|Default|GetPlayerGameDataMap) PlayerController _output_get)
  (bind _keys (Utilities|Map|Keys (Variables|Default|GetPlayerGameDataMap)))
  (for _array_element _keys
    (bind _values (Utilities|Map|Values _playergamedatamap))
    (Default|ClientUpdateAllPlayerHealth _array_element _values)))

(event Custom|RequestSpawn
  (params (PlayerController :type Guardian%20Player%20Controller%20BP%20Object%20Reference))
  ;[1 1 1] Login && Spawn Player
  (Default|SpawnPlayerCharater PlayerController "/Game/BluePrint/Player/Attacker.Attacker_C" (Transformation|GetActorTransform (Utilities|Array|Get(acopy) (Variables|Default|GetCharacter%20Spawn%20Points) (Variables|Default|GetSpawnIndex))))
  (bind _output_get (Variables|Default|SetLife%20Num (- (Variables|Default|GetLife%20Num) 1)))
  (if (< _output_get 0)
    (CallFunction|EndGame)
    (else
      (CallFunction|UpdateLifeNum _output_get)
      (Variables|Default|SetSpawnIndex (+ (Variables|Default|GetSpawnIndex) 1))
      (if (>= (Variables|Default|GetSpawnIndex) (Utilities|Array|Length (Variables|Default|GetCharacter%20Spawn%20Points)))
        (Variables|Default|SetSpawnIndex 0)))))

(event EventPostLogin
  (params (NewPlayer :type Player%20Controller%20Object%20Reference))
  ;[1 1 1] Login && Spawn Player
  (bind _asguardian_player_controller_bp (Utilities|Casting|CastToGuardianPlayerController_BP NewPlayer))
  (if (Variables|Default|GetIsFirstPerson)
    (Variables|Default|SetIsFirstPerson false)
    (CallFunction|UpdateTime))
  (Default|StartSpawnPlayerCharacter _asguardian_player_controller_bp)
  (Variables|Default|SetLife%20Num (+ (Variables|Default|GetLife%20Num) 3))
  (Utilities|Map|Add (Variables|Default|GetPlayerGameDataMap) _asguardian_player_controller_bp (Utilities|Struct|MakeDeathMatchPlayerData (Utilities|String|StringToName (Utilities|GetObjectName _asguardian_player_controller_bp)) 0 0 0 1e+02))
  (CallFunction|SpawAIKata))

(fn ConstructionScript)