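; Player-side Attacker Blueprint that takes weapon damage from AI enemies and drives the first-person arms pose.
; WeaponAttack applies fixed damage to itself with the killer as instigator.
; AnyDamage passes damage to OnHit only when the instigator is a Kata or Shooter AI controller, ignoring other sources.
; UpdateFPArmsBlendPose forwards the new blend index to the client arms animation Blueprint.
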(event Game|Damage|EventAnyDamage
  (params (Damage :type Float%20%28single-precision%29) (DamageType :type Damage%20Type%20Object%20Reference) (InstigatedBy :type Controller%20Object%20Reference) (DamageCauser :type Actor%20Object%20Reference))
  (bind _askata_aicontroller (Utilities|Casting|CastToKataAIController InstigatedBy)
    (:then
      (Class|MyCharacter|OnHit 0 Damage 0 "0, 0, 0" 0 "None" "0, 0, 0" 0 _askata_aicontroller))
    (:CastFailed
      (bind _asshooter_aicontroller (Utilities|Casting|CastToShooterAIController InstigatedBy))
      (Class|MyCharacter|OnHit 0 Damage 0 "0, 0, 0" 0 "None" "0, 0, 0" 0 _asshooter_aicontroller))))

(event EventUpdateFPArmsBlendPose
  (params (NewIndex :type Integer))
  (Class|INTUpdateAnimBlendIndex|UpdateBlendIndex(Message) (Variables|Default|GetClientArmsAnimBP) NewIndex))

(fn ConstructionScript)

(fn WeaponAttack
  (params (Killer :type Kata%20AI%20Controller%20Object%20Reference))
  (Game|Damage|ApplyDamage self 1e+01 Killer 0)
  (return true))